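; BP_Hook is a hook actor where a killer hangs the survivor they are carrying.
; Box overlap by a killer with GrabToSurvivor set shows a trigger prompt widget and opens a gate, which closes when the killer leaves.
; While open, the killer trigger input detaches the survivor found by GetActorOfClass, snaps it to the hook mesh's Point socket and sets HangingOn.
; The actor enables input for player controller 0 on BeginPlay.
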(event OnComponentBeginOverlap(Box)
  (params (OverlappedComponent :type Primitive%20Component%20Object%20Reference) (OtherActor :type Actor%20Object%20Reference) (OtherComp :type Primitive%20Component%20Object%20Reference) (OtherBodyIndex :type Integer) (bFromSweep :type Boolean) (SweepResult :type Hit%20Result%20Structure%20%28by%20ref%29))
  (bind _asbp_killerll (Utilities|Casting|CastToBP_Killerll OtherActor))
  (if (Variables|/Game/Create/GM/BP_Killerll.BP_Killerll_C|GetGrabToSurvivor _asbp_killerll)
    (bind _returnvalue (UserInterface|CreateWidget "/Game/Create/Widget/WG_Trigger_Info.WG_Trigger_Info_C"))
    (UserInterface|Viewport|AddtoPlayerScreen _returnvalue)
    (Utilities|FlowControl|Gate true) ; enters at Open
  ))

(event OnComponentEndOverlap(Box)
  (params (OverlappedComponent :type Primitive%20Component%20Object%20Reference) (OtherActor :type Actor%20Object%20Reference) (OtherComp :type Primitive%20Component%20Object%20Reference) (OtherBodyIndex :type Integer))
  (Utilities|Casting|CastToBP_Killerll OtherActor)
  (Widget|RemovefromParent (stale OnComponentBeginOverlap(Box) _returnvalue))
  (Utilities|FlowControl|Gate true) ; enters at Close
)

(event Custom|Hook)

(event Input|EnhancedActionEvents|EnhancedInputActionIA_Killer_Trigger
  (params (ActionValue :type Boolean) (ElapsedSeconds :type Float%20%28double-precision%29) (TriggeredSeconds :type Float%20%28double-precision%29) (InputAction :type Input%20Action%20Object%20Reference :default "/Game/Create/GM/Input/Killer/IA_Killer_Trigger.IA_Killer_Trigger"))
  (Utilities|FlowControl|Gate true
    (:Exit
      (bind _returnvalue (Actor|GetActorOfClass "/Game/Create/GM/BP_Survivorll.BP_Survivorll_C"))
      (Default|Detach _returnvalue)
      (Transformation|AttachComponentToComponent _returnvalue (Variables|Default|GetSM_Hook) "Point" "SnapToTarget" "SnapToTarget" "SnapToTarget" true)
      (Variables|/Game/Create/GM/BP_Survivorll.BP_Survivorll_C|SetHangingOn _returnvalue true))))

(event EventBeginPlay
  (Input|EnableInput (Game|GetPlayerController 0)))

(fn ConstructionScript)