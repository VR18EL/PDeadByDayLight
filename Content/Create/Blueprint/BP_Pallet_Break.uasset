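; Droppable, breakable pallet: a BP_Live player can tip it over, then a BP_Killer player can destroy it.
; Box overlaps show a trigger prompt and open gates for each role's input, the killer's only after the drop.
; A timeline rotates the pallet bone, and the killer's montage locks input until the actor is destroyed.
; Separate functions enable physics on two groups of pieces for staged breakage, with no caller in these graphs.
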(event OnComponentBeginOverlap(Box)
  (params (OverlappedComponent :type Primitive%20Component%20Object%20Reference) (OtherActor :type Actor%20Object%20Reference) (OtherComp :type Primitive%20Component%20Object%20Reference) (OtherBodyIndex :type Integer) (bFromSweep :type Boolean) (SweepResult :type Hit%20Result%20Structure%20%28by%20ref%29))
  (bind _returnvalue (Game|GetPlayerController 0))
  (if (== (.AsBP%20Live (Utilities|Casting|CastToBP_Live OtherActor)) OtherActor)
    (bind _returnvalue_2 (UserInterface|CreateWidget "/Game/Create/Blueprint/WG_Trigger_Info.WG_Trigger_Info_C"))
    (UserInterface|Viewport|AddtoPlayerScreen _returnvalue_2 1)
    (Utilities|FlowControl|Gate true) ; enters at Open
    (elif (Variables|Default|GetbIsPalletPlay)
      (bind _asbp_killer (Utilities|Casting|CastToBP_Killer OtherActor))
      (bind _output_get (Variables|Default|SetKiller _asbp_killer))
      (bind _returnvalue_3 (UserInterface|CreateWidget "/Game/Create/Blueprint/WG_Trigger_Info.WG_Trigger_Info_C"))
      (UserInterface|Viewport|AddtoPlayerScreen _returnvalue_3)
      (Utilities|FlowControl|Gate true) ; enters at Open
    )))

(event OnComponentEndOverlap(Box)
  (params (OverlappedComponent :type Primitive%20Component%20Object%20Reference) (OtherActor :type Actor%20Object%20Reference) (OtherComp :type Primitive%20Component%20Object%20Reference) (OtherBodyIndex :type Integer))
  (bind _returnvalue (Game|GetPlayerController 0))
  (bind _killer (Variables|Default|GetKiller))
  (if (== (.AsBP%20Live (Utilities|Casting|CastToBP_Live OtherActor)) OtherActor)
    (Widget|RemovefromParent (stale OnComponentBeginOverlap(Box) _returnvalue_2))
    (Utilities|FlowControl|Gate true) ; enters at Close
    (elif (Variables|Default|GetbIsPalletPlay)
      (Utilities|Casting|CastToBP_Killer OtherActor)
      (Widget|RemovefromParent (stale OnComponentBeginOverlap(Box) _returnvalue_3))
      (Utilities|FlowControl|Gate true) ; enters at Close
    )))

(event Input|EnhancedActionEvents|EnhancedInputActionIA_Killer_Trigger
  (params (ActionValue :type Boolean) (ElapsedSeconds :type Float%20%28double-precision%29) (TriggeredSeconds :type Float%20%28double-precision%29) (InputAction :type Input%20Action%20Object%20Reference :default "/Game/Create/GM/Killer/IA_Killer_Trigger.IA_Killer_Trigger"))
  (bind _returnvalue (Game|GetPlayerController 0))
  (bind _killer (Variables|Default|GetKiller))
  (:Started
    (Utilities|FlowControl|Gate true
      (:Exit
        (Animation|Montage|PlayMontage (Variables|/Script/Engine.Character|GetMesh (stale OnComponentBeginOverlap(Box) _output_get)) "/Game/Create/Animation/Killer/Anim_Destroy.Anim_Destroy"
          (:then
            (Input|DisableInput _killer _returnvalue))
          (:OnCompleted
            (Input|EnableInput _killer _returnvalue)
            (Actor|DestroyActor)))))))

(event Input|EnhancedActionEvents|EnhancedInputActionIA_Live_Trigger
  (params (ActionValue :type Boolean) (ElapsedSeconds :type Float%20%28double-precision%29) (TriggeredSeconds :type Float%20%28double-precision%29) (InputAction :type Input%20Action%20Object%20Reference :default "/Game/Create/GM/Live/IA_Live_Trigger.IA_Live_Trigger"))
  (:Started
    (Utilities|FlowControl|Gate true
      (:Exit
        (bind _movespeed (Timeline|PalletMotion Play)
          (:Update
            (Transformation|SetRelativeRotation (Variables|Default|GetPallet_Bone) (Math|Rotator|MakeRotator 0.0 (Math|Float|Lerp 0.0 45.0 _movespeed) 0.0) false false)
            (Variables|Default|SetbIsPalletPlay true)))))))

(event EventBeginPlay
  (Input|EnableInput (Game|GetPlayerController 0))
  (Input|EnableInput (Game|GetPlayerController 1)))

(fn ConstructionScript)

(fn SimulatePhysics
  (params (bSimulate :type Boolean))
  (for _array_element (Components|GetChildrenComponents (Variables|BP_Pallet_Break_C|GetBox (Variables|Default|GetPallet)) false)
    (bind _asstatic_mesh_component (Utilities|Casting|CastToStaticMeshComponent _array_element))
    (Physics|SetSimulatePhysics _asstatic_mesh_component bSimulate)))

(fn SetPhysicsSecondTarget
  (Physics|SetSimulatePhysics (Variables|Default|GetPallet_Sphere_024) true))

(fn SetDestroySecondAction
  (CallFunction|SetPhysicsSecondTarget (Variables|Default|GetPallet)))

(fn SetDestroyFirstAction
  (CallFunction|SetPhysicsFirstTarget (Variables|Default|GetPallet)))

(fn SetPhysicsFirstTarget
  (Physics|SetSimulatePhysics (Variables|Default|GetPallet_Cube_044) true))