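; Gameplay player controller that creates the in-game UI for the local player and relays player list updates to it.
; On BeginPlay it builds WB_InGameUI and adds it to the viewport.
; UpdatePlayerListPC retries on a short delay until that widget is valid, then updates the list and calls ShowPlayerList with false.
; Possess prints the player name from BP_OurGameInstance; unconnected show/hide and test-print nodes remain.
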(event Custom|UpdatePlayerListPC
  (params (PlayerList :type Array%20of%20S%20Player%20Structures))
  (bind _ui_ref (Variables|Default|GetUI_Ref))
  (Utilities|IsValid _ui_ref :!label _label
    (:Is%20Valid
      (Default|UpdatePlayerList _ui_ref PlayerList)
      (Default|ShowPlayerList _ui_ref false))
    (:Is%20Not%20Valid
      (Utilities|FlowControl|Delay 0.1)
      (goto _label))))

(event EventBeginPlay
  (CallFunction|SetUpUI))

(event EventPossess
  (params (PossessedPawn :type Pawn%20Object%20Reference))
  (bind _asbp_our_game_instance (Utilities|Casting|CastToBP_OurGameInstance (Game|GetGameInstance)))
  (Development|PrintString (Utilities|String|ToString(Text) (Variables|/Game/NI/BP_OurGameInstance.BP_OurGameInstance_C|GetPlayerName _asbp_our_game_instance))))

(event Input|KeyboardEvents|Tab
  (params (Key :type Key%20Structure)))

(fn ConstructionScript)

(fn SetUpUI
  (if (Pawn|IsLocalController)
    (bind _returnvalue (Game|ConstructObjectfromClass "/Game/NI/BP_Boarder/WB_InGameUI.WB_InGameUI_C"))
    (bind _output_get (Variables|Default|SetUI_Ref _returnvalue))
    (UserInterface|Viewport|AddtoViewport _output_get 0)))