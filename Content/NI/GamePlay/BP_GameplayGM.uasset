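; BP_GameplayGM is the gameplay GameMode that keeps the connected players' name list in sync.
; PostLogin and logout update AllPCs, then call UpdatePlayerListGM, which rebuilds PlayerList from each pawn's CustomPlayerName and pushes it to every BP_GameplayPC.
; A missing pawn or empty name schedules a 0.2-second timer to rerun the rebuild, while the partial list is still sent.
; PostLogin also prints the GameInstance's PlayerName.
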(event EventBeginPlay)

(event EventTick
  (params (DeltaSeconds :type Float%20%28single-precision%29)))

(event EventPostLogin
  (params (NewPlayer :type Player%20Controller%20Object%20Reference))
  (Utilities|Array|Add (Variables|Default|GetAllPCs) NewPlayer)
  (bind _asbp_our_game_instance (Utilities|Casting|CastToBP_OurGameInstance (Game|GetGameInstance)))
  (Development|PrintString (Utilities|String|ToString(Text) (Variables|/Game/NI/BP_OurGameInstance.BP_OurGameInstance_C|GetPlayerName _asbp_our_game_instance)))
  (CallFunction|UpdatePlayerListGM))

(event EventOnLogout
  (params (ExitingController :type Controller%20Object%20Reference))
  (bind _asplayer_controller (Utilities|Casting|CastToPlayerController ExitingController))
  (Utilities|Array|RemoveItem (Variables|Default|GetAllPCs) _asplayer_controller)
  (CallFunction|UpdatePlayerListGM))

(fn ConstructionScript)

(fn UpdatePlayerListGM
  (Utilities|Array|Clear (Variables|Default|GetPlayerList))
  (for _array_element (Variables|Default|GetAllPCs)
    (Utilities|IsValid (Pawn|GetControlledPawn _array_element)
      (:Is%20Valid
        (if (Utilities|Text|TextIsEmpty (Variables|/Game/ThirdPerson/Blueprints/BP_ThirdPersonCharacter.BP_ThirdPersonCharacter_C|GetCustom%20Player%20Name (.AsBP%20Third%20Person%20Character (Utilities|Casting|CastToBP_ThirdPersonCharacter (Pawn|GetControlledPawn _array_element)))))
          (Utilities|Time|SetTimerbyFunctionName 0 "UpdatePlayerListGM" 0.2 :!label _label)
          (else
            (Utilities|Array|Add (Variables|Default|GetPlayerList) (Utilities|Struct|MakeS_Player (Variables|/Game/ThirdPerson/Blueprints/BP_ThirdPersonCharacter.BP_ThirdPersonCharacter_C|GetCustom%20Player%20Name (.AsBP%20Third%20Person%20Character (Utilities|Casting|CastToBP_ThirdPersonCharacter (Pawn|GetControlledPawn _array_element)))))))))
      (:Is%20Not%20Valid
        (goto _label))))
  (for _array_element_2 (Variables|Default|GetAllPCs)
    (bind _asbp_gameplay_pc (Utilities|Casting|CastToBP_GameplayPC _array_element_2))
    (Default|UpdatePlayerListPC _asbp_gameplay_pc (Variables|Default|GetPlayerList))))