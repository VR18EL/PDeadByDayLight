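; BP_LobbyPlayerPlatform is a lobby slot that displays a player's character and offers a button to open the friend list.
; SpawnCharacter replaces the displayed character, hides the button and closes the friend list if parked here; Clear empties the slot and restores the button.
; On the server, BeginPlay finds the BP_FriendList actor and links the button widget, so ShowFriendList can move that list to this platform.
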(event Custom|SpawnCharacter
  (params (PC :type Player%20Controller%20Object%20Reference))
  (Variables|Default|SetPC PC)
  (Utilities|IsValid (Variables|Default|GetCurentCharacter)
    (:Is%20Valid
      (Actor|DestroyActor (Variables|Default|GetCurentCharacter)))
    (:Is%20Not%20Valid
      _))
  ;[1 1 1] BP(O)이모양은 뭐였을까
  (bind _returnvalue (Game|SpawnActorfromClass "/Game/NI/BP_ThirdPersonCharacter11.BP_ThirdPersonCharacter11_C" (Transformation|GetWorldTransform (Variables|Default|GetPlayerSpawnTransform)) "Undefined" "MultiplyWithRoot" 0 0))
  (Variables|Default|SetCurentCharacter _returnvalue)
  (Rendering|SetVisibility (Variables|Default|GetOpenFriendListButton) false false)
  (if (Utilities|Operators|EqualEqual (Transformation|GetWorldLocation (Variables|Default|GetFriendListLocation)) (Transformation|GetActorLocation (Variables|Default|GetFriendListRef)) 5.0)
    (Default|Show (Variables|Default|GetFriendListRef) false)))

(event Custom|Clear
  (Variables|Default|SetPC 0)
  (Utilities|IsValid (Variables|Default|GetCurentCharacter)
    (:Is%20Valid
      (Actor|DestroyActor (Variables|Default|GetCurentCharacter))
      (Variables|Default|SetCurentCharacter 0))
    (:Is%20Not%20Valid
      _))
  (Rendering|SetVisibility (Variables|Default|GetOpenFriendListButton) true false))

(event EventBeginPlay
  (CallFunction|SetUpServer))

(fn ConstructionScript)

(fn ShowFriendList
  (params (bShow :type Boolean))
  (bind _openfriendlistbutton (Variables|Default|GetOpenFriendListButton))
  (bind _returnvalue (UserInterface|GetWidget _openfriendlistbutton))
  ;[1 1 1] 초대받은사람들은 +가 안보여용
  (if bShow
    (Widget|SetVisibility _returnvalue "Collapsed")
    (Transformation|SetActorLocation (Variables|Default|GetFriendListRef) (Transformation|GetWorldLocation (Variables|Default|GetFriendListLocation)) false false)
    (Default|Show (Variables|Default|GetFriendListRef) true self)
    (else
      (Widget|SetVisibility _returnvalue "Visible"))))

(fn SetUpServer
  ;[1 1 1] 서버에서 친구창 들고오기
  (if (Networking|IsServer)
    (bind _returnvalue (Actor|GetActorOfClass "/Game/NI/Lobby/BP_FriendList.BP_FriendList_C"))
    (Variables|Default|SetFriendListRef _returnvalue)
    (bind _aswb_open_friend_list_button (Utilities|Casting|CastToWB_OpenFriendListButton (UserInterface|GetWidget (Variables|Default|GetOpenFriendListButton))))
    (Variables|/Game/NI/Lobby/WB_OpenFriendListButton.WB_OpenFriendListButton_C|SetLobbyPlayerPlatformRef _aswb_open_friend_list_button self)
    ;[1 1 1] 비지비지블
    (Rendering|SetVisibility (Variables|Default|GetOpenFriendListButton) true false)))