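; BP_PC, apparently a player controller, relays repair progress and completion events for generators and hooks.
; On BeginPlay it binds to the dispatchers of every BP_Generator_Mul and BP_GalProgress, with Call functions wrapping its events.
; Those events add frame delta time to RepairProgress, destroy cleared generators, and enable physics on cleared hook meshes.
; Generator updates also pass through UpdateGenPMulti to set the widget's remaining hold time.
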(event Custom|DestroyGenerator
  (params (Target :type BP%20Generator%20Mul%20Object%20Reference))
  (if (Utilities|IsValid Target)
    (Actor|DestroyActor Target)))

(event Custom|UpdateGenProgress
  (params (TargetP :type Float%20%28double-precision%29) (Target :type BP%20Generator%20Mul%20Object%20Reference))
  (Variables|/Game/DK/BP_Generator_Mul.BP_Generator_Mul_C|SetRepairProgress Target (+ TargetP (Utilities|Time|GetWorldDeltaSeconds)))
  (CallFunction|UpdateGenPMulti Target))

(event Custom|ClearHook
  (params (Target :type BP%20Gal%20Progress%20Object%20Reference))
  (if (Utilities|IsValid Target)
    (Physics|SetSimulatePhysics (Variables|/Game/DK/BP_GalProgress.BP_GalProgress_C|GetSM_Hook Target) true)))

(event Custom|UpdateHookProgress
  (params (Target :type BP%20Gal%20Progress%20Object%20Reference) (Progress :type Float%20%28double-precision%29))
  (Variables|/Game/DK/BP_GalProgress.BP_GalProgress_C|SetRepairProgress Target (+ Progress (Utilities|Time|GetWorldDeltaSeconds))))

(event Custom|UpdateGenPMulti
  (params (Target :type BP%20Generator%20Mul%20Object%20Reference))
  (bind _widgetref (Variables|/Game/DK/BP_Generator_Mul.BP_Generator_Mul_C|GetWidgetREF Target)
    (:then
      (Variables|/Game/ThirdPerson/Blueprints/Survivor/Mission/WBP_MissionProgress.WBP_MissionProgress_C|SetTimeHeld _widgetref (- (Variables|/Game/DK/BP_Generator_Mul.BP_Generator_Mul_C|GetMaxHeldTime Target) (Variables|/Game/DK/BP_Generator_Mul.BP_Generator_Mul_C|GetRepairProgress Target))))
    (:else)))

(event EventBeginPlay
  (Utilities|FlowControl|Sequence
    (:then_0
      (bind _outactors (Actor|GetAllActorsOfClass "/Game/DK/BP_Generator_Mul.BP_Generator_Mul_C"))
      (for _array_element _outactors
        (EventDispatchers|BindEventtoEDClear1 _array_element (EventDispatchers|CreateEvent :!event CallDestroy))
        (EventDispatchers|BindEventtoEDUpdateProgress _array_element (EventDispatchers|CreateEvent :!event CallProgress))))
    (:then_1
      (bind _outactors_2 (Actor|GetAllActorsOfClass "/Game/DK/BP_GalProgress.BP_GalProgress_C"))
      (for _array_element_2 _outactors_2
        (EventDispatchers|BindEventtoEDUpdateGalProgress _array_element_2 (EventDispatchers|CreateEvent :!event CallGalProgress))
        (EventDispatchers|BindEventtoEDClearHook _array_element_2 (EventDispatchers|CreateEvent :!event CallClearHook))))))

(fn ConstructionScript)

(fn CallDestroy
  (params (Target :type BP%20Generator%20Mul%20Object%20Reference))
  (CallFunction|DestroyGenerator Target))

(fn CallProgress
  (params (ServerProgress :type Float%20%28double-precision%29) (TargetGen :type BP%20Generator%20Mul%20Object%20Reference))
  (CallFunction|UpdateGenProgress ServerProgress TargetGen))

(fn CallGalProgress
  (params (Target :type BP%20Gal%20Progress%20Object%20Reference) (ServerProgressHook :type Float%20%28double-precision%29))
  (CallFunction|UpdateHookProgress Target ServerProgressHook))

(fn CallClearHook
  (params (TargetGen :type BP%20Gal%20Progress%20Object%20Reference))
  (CallFunction|ClearHook TargetGen))