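; BP_ExitTest is a mission exit where a locally controlled survivor in its box holds input on a lever to open the doors.
; Overlap, once the mission is clear, enables input and shows a progress widget.
; Holding fires event dispatchers for progress updates and, after the remaining hold time, exit clear.
; RepNotifies light the spotlight and arm the exit, sync lever and widget to progress, and slide three doors open sequentially by timer.
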(event OnComponentBeginOverlap(Box)
  (params (OverlappedComponent :type Primitive%20Component%20Object%20Reference) (OtherActor :type Actor%20Object%20Reference) (OtherComp :type Primitive%20Component%20Object%20Reference) (OtherBodyIndex :type Integer) (bFromSweep :type Boolean) (SweepResult :type Hit%20Result%20Structure%20%28by%20ref%29))
  (if (not (Variables|Default|GetbIsClear))
    (if (Variables|Default|GetbIsClearMission)
      (bind _asbp_test_survivor (Utilities|Casting|CastToBP_TestSurvivor OtherActor))
      (bind _output_get (Variables|Default|SetCurrent%20Player _asbp_test_survivor))
      (if (Pawn|IsLocallyControlled _output_get)
        (Input|EnableInput (Pawn|GetLocalViewingPlayerController (Variables|Default|GetCurrent%20Player)))
        ;[1 1 1] Mission Overlap시 진행도 / 안내문구 Widget 설정
        (bind _returnvalue (Game|ConstructObjectfromClass "/Game/ThirdPerson/Blueprints/Survivor/Mission/WBP_MissionProgress.WBP_MissionProgress_C"))
        (bind _output_get_2 (Variables|Default|SetWidget%20REF _returnvalue))
        (UserInterface|Viewport|AddtoViewport _output_get_2 0)
        (Variables|/Game/ThirdPerson/Blueprints/Survivor/Mission/WBP_MissionProgress.WBP_MissionProgress_C|SetTimeHeld _output_get_2 (- (Variables|Default|GetMaxHeldTime) (Variables|Default|GetExitProgress)))
        (Variables|/Game/ThirdPerson/Blueprints/Survivor/Mission/WBP_MissionProgress.WBP_MissionProgress_C|SetMaxTimeHeld _output_get_2 (Variables|Default|GetMaxHeldTime))
        (Utilities|FlowControl|Gate true) ; enters at Open
      ))))

(event OnComponentEndOverlap(Box)
  (params (OverlappedComponent :type Primitive%20Component%20Object%20Reference) (OtherActor :type Actor%20Object%20Reference) (OtherComp :type Primitive%20Component%20Object%20Reference) (OtherBodyIndex :type Integer))
  (if (not (Variables|Default|GetbIsClear))
    (if (Variables|Default|GetbIsClearMission)
      (bind _asbp_test_survivor (Utilities|Casting|CastToBP_TestSurvivor OtherActor))
      (bind _output_get (Variables|Default|SetCurrent%20Player _asbp_test_survivor))
      (if (Pawn|IsLocallyControlled _output_get)
        (Input|DisableInput (Pawn|GetLocalViewingPlayerController (Variables|Default|GetCurrent%20Player)))
        ;[1 1 1] Mission Overlap시 진행도 / 안내문구 Widget 설정
        (Variables|Default|SetIsHeld false)
        (bind _widget_ref (Variables|Default|GetWidget%20REF)
          (:then
            (Widget|RemovefromParent _widget_ref)
            (Utilities|FlowControl|Gate true) ; enters at Close
          )
          (:else))))))

(event Custom|Timer
  ;[1 1 1] Mission Progress Bar 시간 설정
  (bind _returnvalue (Utilities|Time|SetTimerbyEvent (delegate Custom|Timer) (Variables|Default|GetMaxHeldTime) false false 0.01)))

(event Custom|Stop%20Timer
  ;[1 1 1] Mission Progress Bar 시간 설정
  (Utilities|Time|PauseTimerbyHandle (stale Custom|Timer _returnvalue)))

(event Custom|Update%20Timer
  (bind _exitprogress (Variables|Default|GetExitProgress))
  (bind _maxheldtime (Variables|Default|GetMaxHeldTime))
  (bind _returnvalue (- _maxheldtime _exitprogress))
  ;[1 1 1] Mission Progress Bar 시간 설정
  (if (Variables|Default|GetIsHeld)
    (Variables|/Game/ThirdPerson/Blueprints/Survivor/Mission/WBP_MissionProgress.WBP_MissionProgress_C|SetTimeHeld (Variables|Default|GetWidget%20REF) _returnvalue)
    (Utilities|FlowControl|Delay 0.01)
    (CallFunction|UpdateTimer)
    (else
      (CallFunction|StopTimer)
      (Variables|/Game/ThirdPerson/Blueprints/Survivor/Mission/WBP_MissionProgress.WBP_MissionProgress_C|SetTimeHeld (Variables|Default|GetWidget%20REF) _returnvalue))))

(event Input|EnhancedActionEvents|EnhancedInputActionIA_Live_Trigger
  (params (ActionValue :type Boolean) (ElapsedSeconds :type Float%20%28double-precision%29) (TriggeredSeconds :type Float%20%28double-precision%29) (InputAction :type Input%20Action%20Object%20Reference :default "/Game/Create/GM/Input/Survivor/IA_Live_Trigger.IA_Live_Trigger"))
  (:Triggered
    (if (not (Variables|Default|GetbIsClear))
      (if (Variables|Default|GetIsHeld)
        ;[1 1 1] ED
        (Default|CallEDUdateExitProgress (Variables|Default|GetExitProgress) self))))
  (:Started
    (Variables|Default|SetIsHeld true)
    (Utilities|FlowControl|Gate true
      (:Exit
        ;[1 1 1] Mission Progress Bar
        (Utilities|FlowControl|Sequence
          (:then_0
            (Utilities|FlowControl|RetriggerableDelay (- (Variables|Default|GetMaxHeldTime) (Variables|Default|GetExitProgress)))
            (if (Variables|Default|GetIsHeld)
              (Default|CallEDClearExit self)))
          (:then_1
            (CallFunction|Timer)
            (CallFunction|UpdateTimer))))))
  (:Completed
    (Variables|Default|SetIsHeld false)
    (Utilities|Time|PauseTimerbyHandle)))

(fn ConstructionScript
  (Transformation|AttachComponentToComponent (Variables|Default|GetSM_Exit_Lever_Handle) (Variables|Default|GetSM_Exit_Lever_Body) "Handle" "SnapToTarget" "SnapToTarget" "SnapToTarget" true)
  (Transformation|AttachComponentToComponent (Variables|Default|GetSM_Exit_Gear) (Variables|Default|GetSM_Exit_Top) "Gear" "SnapToTarget" "SnapToTarget" "SnapToTarget" true))

(fn Action
  (if (< (Variables|Default|GetActionValue) 9e+01)
    (Transformation|AddLocalRotation (Variables|Default|GetSM_Exit_Lever_Handle) "0.000000,0.000000,-2.000000" false false)
    (Transformation|AddLocalRotation (Variables|Default|GetSM_Exit_Gear) "2.000000,0.000000,0.000000" false false)
    (bind _result (Math|Float|IncrementFloat (Variables|Default|GetActionValue))
      (:%20%20
        (return _result)))))

(fn DoorOpen
  (if (< (Variables|Default|GetDoor03) 52.0)
    (Transformation|AddLocalOffset (Variables|Default|GetSM_Exit_Door_03) "-6.000000,0.000000,0.000000" false false)
    (Math|Float|IncrementFloat (Variables|Default|GetDoor03))
    (elif (< (Variables|Default|GetDoor02) 52.0)
      (Transformation|AddLocalOffset (Variables|Default|GetSM_Exit_Door_02) "-6.000000,0.000000,0.000000" false false)
      (Math|Float|IncrementFloat (Variables|Default|GetDoor02))
      (elif (< (Variables|Default|GetDoor01) 52.0)
        (Transformation|AddLocalOffset (Variables|Default|GetSM_Exit_Door_01) "-6.000000,0.000000,0.000000" false false)
        (Math|Float|IncrementFloat (Variables|Default|GetDoor01))
        (else
          (Development|PrintString "Clear~!~!")
          (Utilities|Time|ClearTimerbyFunctionName 0 "DoorOpen"))))))

(fn OnRepClearIntensity
  (Rendering|Components|Light|SetIntensity (Variables|Default|GetSpotLight) (Variables|Default|GetClearIntensity))
  (Variables|Default|SetbIsClearMission true))

(fn OnRepBIsClear
  (Utilities|Time|SetTimerbyFunctionName 0 "DoorOpen" 0.05 true)
  (bind _widget_ref (Variables|Default|GetWidget%20REF)
    (:then
      (Widget|RemovefromParent _widget_ref))
    (:else)))

(fn OnRepExitProgress
  (bind _widget_ref (Variables|Default|GetWidget%20REF)
    (:then
      (Variables|/Game/ThirdPerson/Blueprints/Survivor/Mission/WBP_MissionProgress.WBP_MissionProgress_C|SetTimeHeld _widget_ref (- (Variables|Default|GetMaxHeldTime) (Variables|Default|GetExitProgress)))
      (Transformation|SetRelativeRotation (Variables|Default|GetSM_Exit_Lever_Handle) (Math|Rotator|MakeRotator (* (Variables|Default|GetExitProgress) -1.8e+02) 0.0 0.0) false false))
    (:else)))