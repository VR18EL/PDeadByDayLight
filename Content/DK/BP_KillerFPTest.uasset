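; BP_KillerFPTest is a test first-person killer character with Enhanced Input move, look and montage-based attack, and a weapon attached to a hand socket.
; Its Hit function traces briefly from the camera, calls TempHit on a struck survivor, plays a delay montage and records first or second hit.
; On authority, weapon overlap with a twice-hit survivor shows a prompt widget and opens a gate letting Q call CallEDGrap, until overlap ends.
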(event OnComponentBeginOverlap(SM_Weapon)
  (params (OverlappedComponent :type Primitive%20Component%20Object%20Reference) (OtherActor :type Actor%20Object%20Reference) (OtherComp :type Primitive%20Component%20Object%20Reference) (OtherBodyIndex :type Integer) (bFromSweep :type Boolean) (SweepResult :type Hit%20Result%20Structure%20%28by%20ref%29))
  ;[0 0.2 0 0.5 15] Surviver
  (bind _asbp_test_survivor (Utilities|Casting|CastToBP_TestSurvivor OtherActor))
  (bind _output_get (Variables|Default|SetCurrentSurvivor _asbp_test_survivor))
  (if (Variables|/Game/DK/BP_TestSurvivor.BP_TestSurvivor_C|Get2hit? _output_get)
    (Networking|SwitchHasAuthority
      (:Authority
        (bind _returnvalue (Game|ConstructObjectfromClass "/Game/Create/Widget/WG_Trigger_Info.WG_Trigger_Info_C"))
        (bind _output_get_2 (Variables|Default|SetWidget%20REF _returnvalue))
        (UserInterface|Viewport|AddtoViewport _output_get_2 0)
        (Utilities|FlowControl|Gate true) ; enters at Open
      ))))

(event OnComponentEndOverlap(SM_Weapon)
  (params (OverlappedComponent :type Primitive%20Component%20Object%20Reference) (OtherActor :type Actor%20Object%20Reference) (OtherComp :type Primitive%20Component%20Object%20Reference) (OtherBodyIndex :type Integer))
  ;[0 0.2 0 0.5 15] Surviver
  (bind _asbp_test_survivor (Utilities|Casting|CastToBP_TestSurvivor OtherActor))
  (Variables|Default|SetCurrentSurvivor _asbp_test_survivor)
  (Networking|SwitchHasAuthority
    (:Authority
      (bind _widget_ref (Variables|Default|GetWidget%20REF)
        (:then
          (Widget|RemovefromParent _widget_ref)
          (Utilities|FlowControl|Gate true) ; enters at Close
        )
        (:else)))))

(event Custom|Attack
  (Animation|Montage|PlayMontage (Variables|Character|GetMesh) "/Game/DK/Anim_Attack_FP_Test.Anim_Attack_FP_Test"))

(event Input|EnhancedActionEvents|EnhancedInputActionIA_Move
  (params (ActionValue :type Vector%202D%20Structure) (ElapsedSeconds :type Float%20%28double-precision%29) (TriggeredSeconds :type Float%20%28double-precision%29) (InputAction :type Input%20Action%20Object%20Reference :default "/Game/ThirdPerson/Input/Actions/IA_Move.IA_Move"))
  (bind _returnvalue (Pawn|GetControlRotation :!class /Script/Engine.Pawn))
  ;[1 1 1] Movement
  (Pawn|Input|AddMovementInput (Math|Vector|GetRightVector (Math|Rotator|MakeRotator (.roll _returnvalue) 0.0 (.yaw _returnvalue))) (.x ActionValue) false)
  (Pawn|Input|AddMovementInput (Math|Vector|GetForwardVector (Math|Rotator|MakeRotator 0.0 0.0 (.yaw (Pawn|GetControlRotation :!class /Script/Engine.Pawn)))) (.y ActionValue) false))

(event Input|EnhancedActionEvents|EnhancedInputActionIA_Attack
  (params (ActionValue :type Boolean) (ElapsedSeconds :type Float%20%28double-precision%29) (TriggeredSeconds :type Float%20%28double-precision%29) (InputAction :type Input%20Action%20Object%20Reference :default "/Game/Create/GM/Input/Killer/IA_Attack.IA_Attack"))
  (:Started
    (CallFunction|Attack)))

(event Input|EnhancedActionEvents|EnhancedInputActionIA_Look
  (params (ActionValue :type Vector%202D%20Structure) (ElapsedSeconds :type Float%20%28double-precision%29) (TriggeredSeconds :type Float%20%28double-precision%29) (InputAction :type Input%20Action%20Object%20Reference :default "/Game/ThirdPerson/Input/Actions/IA_Look.IA_Look"))
  ;[1 1 1] Camera
  (Pawn|Input|AddControllerYawInput (.x ActionValue))
  (Pawn|Input|AddControllerPitchInput (.y ActionValue)))

(event EventBeginPlay
  ;[1 1 1] Input
  (bind _as플레이어_컨트롤러 (Utilities|Casting|CastToPlayerController (Pawn|GetController)))
  (Utilities|IsValid (PlayerController|LocalPlayerSubsystems|GetEnhancedInputLocalPlayerSubsystem _as플레이어_컨트롤러)
    (:Is%20Valid
      (Input|AddMappingContext (PlayerController|LocalPlayerSubsystems|GetEnhancedInputLocalPlayerSubsystem _as플레이어_컨트롤러) "/Game/Create/GM/Input/IMC_Killer.IMC_Killer" 0 "(bIgnoreAllPressedKeysUntilRelease=True,bForceImmediately=False,bNotifyUserSettings=False)")
      (Input|DisableInput (.AsBP%20PC (Utilities|Casting|CastToBP_PC (Game|GetPlayerController 0))))
      (Rendering|Components|Light|SetIntensity (Variables|Default|GetRedLight) 0.0))))

(event Input|KeyboardEvents|Q
  (params (Key :type Key%20Structure))
  (:Pressed
    ;[0 0.2 0 0.5 15] Surviver
    (Utilities|FlowControl|Gate true
      (:Exit
        (Default|CallEDGrap)))))

(fn ConstructionScript
  (Transformation|AttachComponentToComponent (Variables|Default|GetSM_Weapon) (Variables|Character|GetMesh) "Weapon_Hand" "SnapToTarget" "SnapToTarget" "SnapToTarget" true))

(fn Hit
  (bind _firstpersoncamera (Variables|Default|GetFirstPersonCamera))
  (bind _returnvalue (Transformation|GetWorldLocation _firstpersoncamera))
  (bind _outhit (Collision|LineTraceForObjects _returnvalue (+ _returnvalue (* (Math|Vector|GetForwardVector _firstpersoncamera) 1e+02)) (Utilities|Array|MakeArray "ObjectTypeQuery3" "ObjectTypeQuery1" "ObjectTypeQuery2" "ObjectTypeQuery4") false 0 "None"))
  (bind _asbp_test_survivor (Utilities|Casting|CastToBP_TestSurvivor (.HitActor (Collision|BreakHitResult _outhit))))
  (Default|TempHit _asbp_test_survivor)
  (Animation|PlayAnimMontage "/Game/Create/Animation/Killer/Anim_Attack_Delay.Anim_Attack_Delay" 1.5 "None")
  (if (Variables|Default|GetFirst_Hit)
    (Variables|Default|SetSecond_Hit true)
    (else
      (Variables|Default|SetFirst_Hit true)))
  (return))